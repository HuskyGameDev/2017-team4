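; Enemy spawner actor that spawns a Ghost at its own location and replaces it once it is gone.
; SpawnEnemy selects the class by number (only 0, Ghost, is handled), passes it the Player reference and stores it as SpawnedEnemy.
; Tick uses latent Delays to hold off the first check, then to pause before calling SpawnEnemy whenever SpawnedEnemy is invalid.
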(event Custom|Spawn%20Enemy
  (params (EnemyNumber :type Integer))
  ;[1 1 1] Take in a number
  ;[1 1 1] Spawn the enemy associated with that number
  (switch int EnemyNumber
    (:0
      (bind _returnvalue (Game|SpawnActorfromClass "/Game/DigitalDemon/Blueprints/Ghost.Ghost_C" (Math|Transform|MakeTransform (Variables|Default|Getspawnlocation) "0, 0, 0" "1,1,1") "Undefined" 0 0))
      (Variables|/Game/DigitalDemon/Blueprints/Enemy.Enemy_C|Setplayer _returnvalue (Variables|Default|Getplayer))
      (Variables|Default|SetspawnedEnemy _returnvalue))))

(event EventBeginPlay
  ;[1 1 1] Set the point where the enemy will spawn
  (Variables|Default|Setspawnlocation (Transformation|GetWorldLocation (Variables|Default|GetDefaultSceneRoot))))

(event Collision|EventActorBeginOverlap
  (params (OtherActor :type Actor%20Object%20Reference)))

(event EventTick
  (params (DeltaSeconds :type Float%20%28single-precision%29))
  ;[1 1 1] If spawned enemy is dead spawn new enemy
  ;;[1 1 1] If first time checking enemy probably hasnt spwaned yet so wait
  (if (Variables|Default|GetfirstCheck)
    (Utilities|FlowControl|Delay 1e+01)
    (Variables|Default|SetfirstCheck false)
    (elif (not (Utilities|IsValid (Variables|Default|GetspawnedEnemy)))
      (Utilities|FlowControl|Delay 2.0)
      (CallFunction|SpawnEnemy))))

(fn ConstructionScript)