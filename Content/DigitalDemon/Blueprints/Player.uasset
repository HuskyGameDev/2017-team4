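; Player Blueprint for an Active Time Battle (ATB) style combatant with health and a charge gauge.
; BeginPlay creates the PlayerATB widget and initializes health, while Tick uses a Delay to steadily fill the gauge's progress bar.
; Damageme subtracts health and updates the HP text while health stays positive; death is unhandled.
; The full-charge check triggers nothing, as the enemy-attack and gauge-reset logic is disconnected.
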(event Custom|Damage%20me
  (params (Damage%20In :type Integer))
  ;[1 1 1] Damage Handling
  (bind _output_get (Variables|Default|SetcurrentHealth (- (Variables|Default|GetcurrentHealth) Damage%20In)))
  (if (not (<= _output_get 0))
    (Rendering|Components|TextRender|SetText (Variables|/Game/DigitalDemon/Blueprints/PlayerATB.PlayerATB_C|GetHPText (Variables|Default|Getatb)) (Utilities|Text|ToText(Integer) (Variables|Default|GetcurrentHealth)))))

(event EventBeginPlay
  ;[1 1 1] Create the Widget
  (bind _returnvalue (UserInterface|CreateWidget "/Game/DigitalDemon/Blueprints/PlayerATB.PlayerATB_C"))
  (bind _output_get (Variables|Default|Setatb _returnvalue))
  (UserInterface|Viewport|AddtoViewport _output_get 0)
  (Rendering|Components|TextRender|SetText (Variables|/Game/DigitalDemon/Blueprints/PlayerATB.PlayerATB_C|GetHPText (Variables|Default|Getatb)) (Utilities|Text|ToText(Integer) (Variables|Default|GetmaxHealth)))
  (Variables|Default|SetcurrentHealth (Variables|Default|GetmaxHealth)))

(event Collision|EventActorBeginOverlap
  (params (OtherActor :type Actor%20Object%20Reference)))

(event EventTick
  (params (DeltaSeconds :type Float%20%28single-precision%29))
  ;[1 1 1] ATB Charging
  (Utilities|FlowControl|Delay 0.1)
  (bind _output_get (Variables|Default|SetatbPercent (+ (Variables|Default|GetatbPercent) 1.25)))
  (Progress|SetPercent (Variables|/Game/DigitalDemon/Blueprints/PlayerATB.PlayerATB_C|GetScorpionHealth (Variables|Default|Getatb)) (/ _output_get 1e+02))
  ;[1 1 1] If ATB is fully charged damage enemy
  (if (== (/ (Variables|Default|GetatbPercent) 1e+02) 1.0)
    _))

(fn ConstructionScript)