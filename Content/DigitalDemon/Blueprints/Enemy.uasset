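; Enemy Blueprint for ATB-style combat that attacks the player on a charge timer and can be damaged and killed.
; BeginPlay creates its EnemyATB widget and initialises HP; a Delay on Tick steps the charge, shown on the ScorpionHealth bar.
; A full bar, tested by exact float equality, calls DamageMe on Player and resets.
; Its own DamageMe updates HP text, removing widget and actor at zero or below.
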(event Custom|Damage%20Me
  (params (damageIn :type Integer))
  (bind _atb (Variables|Default|Getatb))
  (bind _hptext (Variables|/Game/DigitalDemon/Blueprints/EnemyATB.EnemyATB_C|GetHPText _atb))
  ;[1 1 1] Damage Handling
  ;;[1 1 1] Subtract The Damage in from your current health
  (bind _output_get (Variables|Default|SetcurrentHP (- (Variables|Default|GetcurrentHP) damageIn)))
  ;;[1 1 1] Check if health <= 0
  (if (<= _output_get 0)
    ;;[1 1 1] Set health to zero, remove atb, destroy actor
    (Rendering|Components|TextRender|SetText _hptext (Utilities|Text|ToText(Integer) (Variables|Default|GetcurrentHP)))
    (Widget|RemovefromParent (Variables|Default|Getatb))
    (Actor|DestroyActor)
    (else
      ;;[1 1 1] Set health to current hp
      (Rendering|Components|TextRender|SetText _hptext (Utilities|Text|ToText(Integer) (Variables|Default|GetcurrentHP))))))

(event EventBeginPlay
  ;[1 1 1] Create the ATB Widget
  (bind _returnvalue (UserInterface|CreateWidget "/Game/DigitalDemon/Blueprints/EnemyATB.EnemyATB_C"))
  (bind _output_get (Variables|Default|Setatb _returnvalue))
  (UserInterface|Viewport|AddtoViewport _output_get 0)
  ;[1 1 1] Set HP Text to max HP
  (Rendering|Components|TextRender|SetText (Variables|/Game/DigitalDemon/Blueprints/EnemyATB.EnemyATB_C|GetHPText (Variables|Default|Getatb)) (Utilities|Text|ToText(Integer) (Variables|Default|GetmaxHP)))
  ;[1 1 1] Set Current Hp to Max HP
  (Variables|Default|SetcurrentHP (Variables|Default|GetmaxHP)))

(event Collision|EventActorBeginOverlap
  (params (OtherActor :type Actor%20Object%20Reference)))

(event EventTick
  (params (DeltaSeconds :type Float%20%28single-precision%29))
  ;[1 1 1] ATB Charging
  (Utilities|FlowControl|Delay 0.1)
  (bind _output_get (Variables|Default|SetatbPercent (+ (Variables|Default|GetatbPercent) 1.25)))
  (Progress|SetPercent (Variables|/Game/DigitalDemon/Blueprints/EnemyATB.EnemyATB_C|GetScorpionHealth (Variables|Default|Getatb)) (/ _output_get 1e+02))
  ;[1 1 1] If ATB is fully charged damage the player
  (if (== (/ (Variables|Default|GetatbPercent) 1e+02) 1.0)
    (Default|DamageMe (Variables|Default|Getplayer) (Variables|Default|GetmyDamage))
    (bind _output_get_2 (Variables|Default|SetatbPercent 0.0))
    (Progress|SetPercent (Variables|/Game/DigitalDemon/Blueprints/EnemyATB.EnemyATB_C|GetScorpionHealth (Variables|Default|Getatb)) (/ _output_get_2 1e+02))))

(fn ConstructionScript)