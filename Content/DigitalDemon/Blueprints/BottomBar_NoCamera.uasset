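; Four-lane rhythm-game pawn that possesses itself on BeginPlay and points the view at a Backround target.
; StartSong plays the track after a short delay while SpawnNextNote re-calls itself through per-song timing and key arrays, spawning colored notes above their detectors.
; Detector overlaps open hit windows: timely input increments Sucesses, while a missed exit calls still-empty failure events.
; Keys F, S and G start song 1, spawn test notes and print hits.
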(event OnComponentBeginOverlap(Note1Detector)
  (params (OverlappedComponent :type Primitive%20Component%20Object%20Reference) (OtherActor :type Actor%20Object%20Reference) (OtherComp :type Primitive%20Component%20Object%20Reference) (OtherBodyIndex :type Integer) (bFromSweep :type Boolean) (SweepResult :type Hit%20Result%20Structure%20%28by%20ref%29))
  ;[1 1 1] Note1 Flow
  ;;[1 1 1] If a note overlaps Note1Detector set Note1Ready
  (Variables|Default|SetNote1Ready true))

(event OnComponentEndOverlap(Note1Detector)
  (params (OverlappedComponent :type Primitive%20Component%20Object%20Reference) (OtherActor :type Actor%20Object%20Reference) (OtherComp :type Primitive%20Component%20Object%20Reference) (OtherBodyIndex :type Integer))
  ;[1 1 1] Note1 Flow
  ;;[1 1 1] If note stops overlapping Note1Detector and the proper trigger hasn't occured trigger failure
  (if (Variables|Default|GetNote1Ready)
    (Variables|Default|SetNote1Ready false)
    (CallFunction|Note1Failure)))

(event OnComponentBeginOverlap(Note2Detector)
  (params (OverlappedComponent :type Primitive%20Component%20Object%20Reference) (OtherActor :type Actor%20Object%20Reference) (OtherComp :type Primitive%20Component%20Object%20Reference) (OtherBodyIndex :type Integer) (bFromSweep :type Boolean) (SweepResult :type Hit%20Result%20Structure%20%28by%20ref%29))
  ;[1 1 1] Note2 Flow
  ;;[1 1 1] If note overlaps Note2Detector set Note2Ready
  (Variables|Default|SetNote2Ready true))

(event OnComponentEndOverlap(Note2Detector)
  (params (OverlappedComponent :type Primitive%20Component%20Object%20Reference) (OtherActor :type Actor%20Object%20Reference) (OtherComp :type Primitive%20Component%20Object%20Reference) (OtherBodyIndex :type Integer))
  ;[1 1 1] Note2 Flow
  ;;[1 1 1] If note stops overlapping Note2Detector and proper trigger hasn't occured trigger failure
  (if (Variables|Default|GetNote2Ready)
    (Variables|Default|SetNote2Ready false)
    (CallFunction|Note2Failure)))

(event OnComponentBeginOverlap(Note3Detector)
  (params (OverlappedComponent :type Primitive%20Component%20Object%20Reference) (OtherActor :type Actor%20Object%20Reference) (OtherComp :type Primitive%20Component%20Object%20Reference) (OtherBodyIndex :type Integer) (bFromSweep :type Boolean) (SweepResult :type Hit%20Result%20Structure%20%28by%20ref%29))
  ;[1 1 1] Note3 Flow
  ;;[1 1 1] If a note overlaps Note3Detector set Note3Ready
  (Variables|Default|SetNote3Ready true))

(event OnComponentEndOverlap(Note3Detector)
  (params (OverlappedComponent :type Primitive%20Component%20Object%20Reference) (OtherActor :type Actor%20Object%20Reference) (OtherComp :type Primitive%20Component%20Object%20Reference) (OtherBodyIndex :type Integer))
  ;[1 1 1] Note3 Flow
  ;;[1 1 1] If note stops overlapping Note3Detector and the proper trigger hasn't occured, trigger failure
  (if (Variables|Default|GetNote3Ready)
    (Variables|Default|SetNote3Ready false)
    (CallFunction|Note3Failure)))

(event OnComponentBeginOverlap(Note4Detector)
  (params (OverlappedComponent :type Primitive%20Component%20Object%20Reference) (OtherActor :type Actor%20Object%20Reference) (OtherComp :type Primitive%20Component%20Object%20Reference) (OtherBodyIndex :type Integer) (bFromSweep :type Boolean) (SweepResult :type Hit%20Result%20Structure%20%28by%20ref%29))
  ;[1 1 1] Note4 Flow
  ;;[1 1 1] If note overlaps Note4Detector set Note4Ready
  (Variables|Default|SetNote4Ready true))

(event OnComponentEndOverlap(Note4Detector)
  (params (OverlappedComponent :type Primitive%20Component%20Object%20Reference) (OtherActor :type Actor%20Object%20Reference) (OtherComp :type Primitive%20Component%20Object%20Reference) (OtherBodyIndex :type Integer))
  ;[1 1 1] Note4 Flow
  ;;[1 1 1] If note stops overlapping Note4Detector and proper trigger hasn't occered, trigger failure
  (if (Variables|Default|GetNote4Ready)
    (Variables|Default|SetNote4Ready false)
    (CallFunction|Note4Failure)))

(event Custom|Note1Sucess
  ;[1 1 1] Note1 Flow
  ;;[1 1 1] What to Do on Note1 Sucess
  (Math|Integer|IncrementInt (Variables|Default|Getsucesses)))

(event Custom|Note1Failure
  ;[1 1 1] Note1 Flow
  ;;[1 1 1] What to Do on Note1 Failure
)

(event Custom|Note4%20Sucess
  ;[1 1 1] Note4 Flow
  ;;[1 1 1] What to do on Note4 Sucess
  (Math|Integer|IncrementInt (Variables|Default|Getsucesses)))

(event Custom|Note4%20Failure
  ;[1 1 1] Note4 Flow
  ;;[1 1 1] What to do on Note4 Failure
)

(event Custom|Spawn%20Note1
  ;[1 1 1] Note Spawning
  ;;[1 1 1] Spawn note in Note1 column
  (bind _returnvalue (Game|SpawnActorfromClass "/Game/DigitalDemon/Blueprints/Cyan_Note.Cyan_Note_C" (Math|Conversions|ToTransform(Vector) (+ (Transformation|GetSocketLocation (Variables|Default|GetNote1Detector) "None") "0, 0,770.000000")) "Undefined" 0 0))
  (Variables|/Game/DigitalDemon/Blueprints/Cyan_Note.Cyan_Note_C|SetendPoint _returnvalue "0, 0,-861.000000"))

(event Custom|Spawn%20Note3
  ;[1 1 1] Note Spawning
  ;;[1 1 1] Spawn note in Note3 column
  (bind _returnvalue (Game|SpawnActorfromClass "/Game/DigitalDemon/Blueprints/Orange_Note.Orange_Note_C" (Math|Conversions|ToTransform(Vector) (+ (Transformation|GetSocketLocation (Variables|Default|GetNote3Detector) "None") "0, 0,770.000000")) "Undefined" 0 0))
  (Variables|/Game/DigitalDemon/Blueprints/Orange_Note.Orange_Note_C|SetendPoint _returnvalue "0, 0,-861.000000"))

(event Custom|Spawn%20Note2
  ;[1 1 1] Note Spawning
  ;;[1 1 1] Spawn note in Note2 column
  (bind _returnvalue (Game|SpawnActorfromClass "/Game/DigitalDemon/Blueprints/Magenta_note.Magenta_note_C" (Math|Conversions|ToTransform(Vector) (+ (Transformation|GetSocketLocation (Variables|Default|GetNote2Detector) "None") "0, 0,770.000000")) "Undefined" 0 0))
  (Variables|/Game/DigitalDemon/Blueprints/Magenta_note.Magenta_note_C|SetendPoint _returnvalue "0, 0,-861.000000"))

(event Custom|Spawn%20Note4
  ;[1 1 1] Note Spawning
  ;;[1 1 1] Spawn note in Note4 column
  (bind _returnvalue (Game|SpawnActorfromClass "/Game/DigitalDemon/Blueprints/Yellow_Note.Yellow_Note_C" (Math|Conversions|ToTransform(Vector) (+ (Transformation|GetSocketLocation (Variables|Default|GetNote4Detector) "None") "0, 0,770.000000")) "Undefined" 0 0))
  (Variables|/Game/DigitalDemon/Blueprints/Yellow_Note.Yellow_Note_C|SetendPoint _returnvalue "0, 0,-861.000000"))

(event Custom|Note2Sucess
  ;[1 1 1] Note2 Flow
  ;;[1 1 1] What to do on Note2 Sucess
  (Math|Integer|IncrementInt (Variables|Default|Getsucesses)))

(event Custom|Note2%20Failure
  ;[1 1 1] Note2 Flow
  ;;[1 1 1] What to do on Note2 Failure
)

(event Custom|Start%20Song
  (params (SongNumber :type Integer))
  ;[1 1 1] Start Of Song Handling
  (Utilities|FlowControl|Sequence
    (:then_0
      ;;[1 1 1] Set Song Number
      (Variables|Default|SetsongNumber SongNumber))
    (:then_1
      (Utilities|FlowControl|Delay 1.3)
      ;;[1 1 1] Start the Desired Song Here
      (Audio|PlaySound2D (Utilities|Array|Get(acopy) (Variables|Default|Getsongs) (Variables|Default|GetsongNumber))))
    (:then_2
      ;;[1 1 1] Start Spawning of Notes
      (CallFunction|SpawnNextNote))))

(event Custom|Spawn%20Next%20Note
  (bind _notelayout (Variables|Default|GetNoteLayout))
  (bind _songnumber (Variables|Default|GetsongNumber))
  (bind _output (Utilities|Array|Get(acopy) _notelayout _songnumber))
  (bind (_key _time) (Utilities|Struct|BreakNoteLayout _output))
  ;[1 1 1] Handle Song Note Spawning
  (Utilities|FlowControl|Delay (/ (Math|Conversions|ToFloat(Integer) (Utilities|Array|Get(acopy) _time (Variables|Default|Getcounter))) 1e+03))
  (switch int (Utilities|Array|Get(acopy) _key (Variables|Default|Getcounter))
    (:1
      (CallFunction|SpawnNote1))
    (:2
      (CallFunction|SpawnNote2))
    (:3
      (CallFunction|SpawnNote3))
    (:4
      (CallFunction|SpawnNote4)))
  (if (Variables|Default|Getdebug)
    (Development|PrintString (Utilities|String|ToString(Integer) (Variables|Default|Getcounter))))
  (bind _result (Math|Integer|IncrementInt (Variables|Default|Getcounter))
    (:%20%20
      (if (== _result (Utilities|Array|Length _key))
        (Variables|Default|Setcounter 0)
        (else
          (CallFunction|SpawnNextNote))))))

(event Custom|Note3%20Sucess
  ;[1 1 1] Note3 Flow
  ;;[1 1 1] What to do on Note3 Sucess
  (Math|Integer|IncrementInt (Variables|Default|Getsucesses)))

(event Custom|Note3%20Failure
  ;[1 1 1] Note3 Flow
  ;;[1 1 1] What to Do on Note3 Failure
)

(event EventBeginPlay
  (bind _returnvalue (Game|GetPlayerController 0))
  ;[1 1 1] Take Control of the Player Controller to accept inputs
  (Pawn|UnPossess _returnvalue)
  (Pawn|Possess _returnvalue self)
  (Game|Player|SetViewTargetwithBlend _returnvalue (Variables|Default|GetBackround) 0.0 "VTBlend_Linear" 0.0 false))

(event Input|ActionEvents|InputActionNote1
  (params (Key :type Key%20Structure))
  ;[1 1 1] Note1 Flow
  ;;[1 1 1] If Note1 input is pressed and Note1 Ready, Trigger Note 1 sucess
  (:Pressed
    (if (Variables|Default|GetNote1Ready)
      (if (Variables|Default|Getdebug)
        (Development|PrintString "Note1"))
      (Variables|Default|SetNote1Ready false)
      (CallFunction|Note1Sucess))))

(event Input|ActionEvents|InputActionNote2
  (params (Key :type Key%20Structure))
  ;[1 1 1] Note2 Flow
  ;;[1 1 1] If Note2 input is pressed and Note2 Ready, Trigger Note2 sucess
  (:Pressed
    (if (Variables|Default|GetNote2Ready)
      (if (Variables|Default|Getdebug)
        (Development|PrintString "Note2"))
      (Variables|Default|SetNote2Ready false)
      (CallFunction|Note2Sucess))))

(event Input|ActionEvents|InputActionNote3
  (params (Key :type Key%20Structure))
  ;[1 1 1] Note3 Flow
  ;;[1 1 1] If Note3 input is pressed and Note3 Ready, Trigger Note3 sucess
  (:Pressed
    (if (Variables|Default|GetNote3Ready)
      (if (Variables|Default|Getdebug)
        (Development|PrintString "Note3"))
      (Variables|Default|SetNote3Ready false)
      (CallFunction|Note3Sucess))))

(event Input|ActionEvents|InputActionNote4
  (params (Key :type Key%20Structure))
  ;[1 1 1] Note4 Flow
  ;;[1 1 1] If Note4 input is pressed and Note4 Ready, Trigger Note4 sucess
  (:Pressed
    (if (Variables|Default|GetNote4Ready)
      (if (Variables|Default|Getdebug)
        (Development|PrintString "Note4"))
      (Variables|Default|SetNote4Ready false)
      (CallFunction|Note4Sucess))))

(event Input|KeyboardEvents|G
  (params (Key :type Key%20Structure))
  ;[1 1 1] Print Number of Sucessful Hits
  (:Pressed
    (Development|PrintString (Utilities|String|ToString(Integer) (Variables|Default|Getsucesses)))))

(event Input|KeyboardEvents|S
  (params (Key :type Key%20Structure))
  ;[1 1 1] Spawn 4 notes when 's' is pressed
  (:Pressed
    (bind _returnvalue (Game|SpawnActorfromClass "/Game/DigitalDemon/Blueprints/Note.Note_C" (Math|Conversions|ToTransform(Vector) (+ (Transformation|GetSocketLocation (Variables|Default|GetNote1Detector) "None") "0, 0,770.000000")) "Undefined" 0 0))
    (Variables|/Game/DigitalDemon/Blueprints/Note.Note_C|SetendPoint _returnvalue "0, 0,-861.000000")
    (Utilities|FlowControl|Delay 1.0)
    (bind _returnvalue_2 (Game|SpawnActorfromClass "/Game/DigitalDemon/Blueprints/Note.Note_C" (Math|Conversions|ToTransform(Vector) (+ (Transformation|GetSocketLocation (Variables|Default|GetNote2Detector) "None") "0, 0,770.000000")) "Undefined" 0 0))
    (Variables|/Game/DigitalDemon/Blueprints/Note.Note_C|SetendPoint _returnvalue_2 "0, 0,-861.000000")
    (Utilities|FlowControl|Delay 1.0)
    (bind _returnvalue_3 (Game|SpawnActorfromClass "/Game/DigitalDemon/Blueprints/Note.Note_C" (Math|Conversions|ToTransform(Vector) (+ (Transformation|GetSocketLocation (Variables|Default|GetNote3Detector) "None") "0, 0,770.000000")) "Undefined" 0 0))
    (Variables|/Game/DigitalDemon/Blueprints/Note.Note_C|SetendPoint _returnvalue_3 "0, 0,-861.000000")
    (Utilities|FlowControl|Delay 0.2)
    (bind _returnvalue_4 (Game|SpawnActorfromClass "/Game/DigitalDemon/Blueprints/Note.Note_C" (Math|Conversions|ToTransform(Vector) (+ (Transformation|GetSocketLocation (Variables|Default|GetNote4Detector) "None") "0, 0,770.000000")) "Undefined" 0 0))
    (Variables|/Game/DigitalDemon/Blueprints/Note.Note_C|SetendPoint _returnvalue_4 "0, 0,-861.000000")))

(event Input|KeyboardEvents|F
  (params (Key :type Key%20Structure))
  ;[1 1 1] Start Of Song Handling
  (:Pressed
    (CallFunction|StartSong 1)))

(fn ConstructionScript)