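; BottomBar is a pawn that acts as the hit bar for a four-lane note-timing game, possessed by the first player controller on BeginPlay.
; Each lane's detector sets a ready flag while overlapped, and the matching input action consumes it and prints the note's name.
; Ending an overlap clears an unconsumed flag, but only lane 1 reports failure or success.
; All feedback is debug print strings, with no scoring.
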(event OnComponentBeginOverlap(Note1Detector)
  (params (OverlappedComponent :type Primitive%20Component%20Object%20Reference) (OtherActor :type Actor%20Object%20Reference) (OtherComp :type Primitive%20Component%20Object%20Reference) (OtherBodyIndex :type Integer) (bFromSweep :type Boolean) (SweepResult :type Hit%20Result%20Structure%20%28by%20ref%29))
  (Variables|Default|SetNote1Ready true))

(event OnComponentEndOverlap(Note1Detector)
  (params (OverlappedComponent :type Primitive%20Component%20Object%20Reference) (OtherActor :type Actor%20Object%20Reference) (OtherComp :type Primitive%20Component%20Object%20Reference) (OtherBodyIndex :type Integer))
  (if (Variables|Default|GetNote1Ready)
    (Variables|Default|SetNote1Ready false)
    (Development|PrintString "Fail")
    (else
      (Development|PrintString "Sucess"))))

(event OnComponentBeginOverlap(Note2Detector)
  (params (OverlappedComponent :type Primitive%20Component%20Object%20Reference) (OtherActor :type Actor%20Object%20Reference) (OtherComp :type Primitive%20Component%20Object%20Reference) (OtherBodyIndex :type Integer) (bFromSweep :type Boolean) (SweepResult :type Hit%20Result%20Structure%20%28by%20ref%29))
  (Variables|Default|SetNote2Ready true))

(event OnComponentEndOverlap(Note2Detector)
  (params (OverlappedComponent :type Primitive%20Component%20Object%20Reference) (OtherActor :type Actor%20Object%20Reference) (OtherComp :type Primitive%20Component%20Object%20Reference) (OtherBodyIndex :type Integer))
  (if (Variables|Default|GetNote2Ready)
    (Variables|Default|SetNote2Ready false)))

(event OnComponentBeginOverlap(Note3Detector)
  (params (OverlappedComponent :type Primitive%20Component%20Object%20Reference) (OtherActor :type Actor%20Object%20Reference) (OtherComp :type Primitive%20Component%20Object%20Reference) (OtherBodyIndex :type Integer) (bFromSweep :type Boolean) (SweepResult :type Hit%20Result%20Structure%20%28by%20ref%29))
  (Variables|Default|SetNote3Ready true))

(event OnComponentEndOverlap(Note3Detector)
  (params (OverlappedComponent :type Primitive%20Component%20Object%20Reference) (OtherActor :type Actor%20Object%20Reference) (OtherComp :type Primitive%20Component%20Object%20Reference) (OtherBodyIndex :type Integer))
  (if (Variables|Default|GetNote3Ready)
    (Variables|Default|SetNote3Ready false)))

(event OnComponentBeginOverlap(Note4Detector)
  (params (OverlappedComponent :type Primitive%20Component%20Object%20Reference) (OtherActor :type Actor%20Object%20Reference) (OtherComp :type Primitive%20Component%20Object%20Reference) (OtherBodyIndex :type Integer) (bFromSweep :type Boolean) (SweepResult :type Hit%20Result%20Structure%20%28by%20ref%29))
  (Variables|Default|SetNote4Ready true))

(event OnComponentEndOverlap(Note4Detector)
  (params (OverlappedComponent :type Primitive%20Component%20Object%20Reference) (OtherActor :type Actor%20Object%20Reference) (OtherComp :type Primitive%20Component%20Object%20Reference) (OtherBodyIndex :type Integer))
  (if (Variables|Default|GetNote4Ready)
    (Variables|Default|SetNote4Ready false)))

(event EventBeginPlay
  (bind _returnvalue (Game|GetPlayerController 0))
  (Pawn|UnPossess _returnvalue)
  (Pawn|Possess _returnvalue self))

(event Input|ActionEvents|InputActionNote1
  (params (Key :type Key%20Structure))
  (:Pressed
    (if (Variables|Default|GetNote1Ready)
      (Development|PrintString "Note1")
      (Variables|Default|SetNote1Ready false))))

(event Input|ActionEvents|InputActionNote2
  (params (Key :type Key%20Structure))
  (:Pressed
    (if (Variables|Default|GetNote2Ready)
      (Development|PrintString "Note2")
      (Variables|Default|SetNote2Ready false))))

(event Input|ActionEvents|InputActionNote3
  (params (Key :type Key%20Structure))
  (:Pressed
    (if (Variables|Default|GetNote3Ready)
      (Development|PrintString "Note3")
      (Variables|Default|SetNote3Ready false))))

(event Input|ActionEvents|InputActionNote4
  (params (Key :type Key%20Structure))
  (:Pressed
    (if (Variables|Default|GetNote4Ready)
      (Development|PrintString "Note4")
      (Variables|Default|SetNote4Ready false))))

(fn ConstructionScript)