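; Yellow note actor that travels from its relative origin to an end point, then destroys itself.
; On BeginPlay it sets the timeline play rate to the inverse of Speed, so Speed acts as a duration scale.
; FallTimeline lerps the Note component's relative location to EndPoint, and the actor is destroyed shortly after it finishes.
; A leftover branch that spawns a replacement note is disconnected and never runs.
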(event Custom|Moving%20Forward
  ;[1 1 1] Movement Control
  (bind _newtrack_0 (Timeline|FallTimeline PlayFromStart)
    (:Update
      (Transformation|SetRelativeLocation (Variables|Default|GetNote) (Math|Vector|Lerp(Vector) "0, 0, 0" (Variables|Default|GetendPoint) _newtrack_0) false false))
    (:Finished
      (Utilities|FlowControl|Delay 0.2)
      (Actor|DestroyActor))))

(event EventBeginPlay
  (Utilities|FlowControl|Sequence
    (:then_1
      (Components|Timeline|SetPlayRate (Variables|Default|GetFallTimeline) (/ 1.0 (Variables|Default|Getspeed)))
      (Variables|Default|SettestEnd true)
      (CallFunction|MovingForward))))

(event Collision|EventActorBeginOverlap
  (params (OtherActor :type Actor%20Object%20Reference)))

(event EventTick
  (params (DeltaSeconds :type Float%20%28single-precision%29)))

(fn ConstructionScript)