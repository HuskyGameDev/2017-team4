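; AndysBar is a possessable rhythm-game note bar that the player controller possesses on BeginPlay.
; Pressing S spawns four timed Note actors above four detectors with downward end points.
; Detector overlaps arm per-lane ready flags that note inputs consume; only lane one prints fail or success.
; Next and Prev Action inputs cycle the ATK, DEF and EVA HUD widgets.
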(event OnComponentBeginOverlap(Note1Detector)
  (params (OverlappedComponent :type Primitive%20Component%20Object%20Reference) (OtherActor :type Actor%20Object%20Reference) (OtherComp :type Primitive%20Component%20Object%20Reference) (OtherBodyIndex :type Integer) (bFromSweep :type Boolean) (SweepResult :type Hit%20Result%20Structure%20%28by%20ref%29))
  (Variables|Default|SetNote1Ready true))

(event OnComponentEndOverlap(Note1Detector)
  (params (OverlappedComponent :type Primitive%20Component%20Object%20Reference) (OtherActor :type Actor%20Object%20Reference) (OtherComp :type Primitive%20Component%20Object%20Reference) (OtherBodyIndex :type Integer))
  (if (Variables|Default|GetNote1Ready)
    (Variables|Default|SetNote1Ready false)
    (Development|PrintString "Fail")
    (else
      (Development|PrintString "Sucess"))))

(event OnComponentBeginOverlap(Note2Detector)
  (params (OverlappedComponent :type Primitive%20Component%20Object%20Reference) (OtherActor :type Actor%20Object%20Reference) (OtherComp :type Primitive%20Component%20Object%20Reference) (OtherBodyIndex :type Integer) (bFromSweep :type Boolean) (SweepResult :type Hit%20Result%20Structure%20%28by%20ref%29))
  (Variables|Default|SetNote2Ready true))

(event OnComponentEndOverlap(Note2Detector)
  (params (OverlappedComponent :type Primitive%20Component%20Object%20Reference) (OtherActor :type Actor%20Object%20Reference) (OtherComp :type Primitive%20Component%20Object%20Reference) (OtherBodyIndex :type Integer))
  (if (Variables|Default|GetNote2Ready)
    (Variables|Default|SetNote2Ready false)))

(event OnComponentBeginOverlap(Note3Detector)
  (params (OverlappedComponent :type Primitive%20Component%20Object%20Reference) (OtherActor :type Actor%20Object%20Reference) (OtherComp :type Primitive%20Component%20Object%20Reference) (OtherBodyIndex :type Integer) (bFromSweep :type Boolean) (SweepResult :type Hit%20Result%20Structure%20%28by%20ref%29))
  (Variables|Default|SetNote3Ready true))

(event OnComponentEndOverlap(Note3Detector)
  (params (OverlappedComponent :type Primitive%20Component%20Object%20Reference) (OtherActor :type Actor%20Object%20Reference) (OtherComp :type Primitive%20Component%20Object%20Reference) (OtherBodyIndex :type Integer))
  (if (Variables|Default|GetNote3Ready)
    (Variables|Default|SetNote3Ready false)))

(event OnComponentBeginOverlap(Note4Detector)
  (params (OverlappedComponent :type Primitive%20Component%20Object%20Reference) (OtherActor :type Actor%20Object%20Reference) (OtherComp :type Primitive%20Component%20Object%20Reference) (OtherBodyIndex :type Integer) (bFromSweep :type Boolean) (SweepResult :type Hit%20Result%20Structure%20%28by%20ref%29))
  (Variables|Default|SetNote4Ready true))

(event OnComponentEndOverlap(Note4Detector)
  (params (OverlappedComponent :type Primitive%20Component%20Object%20Reference) (OtherActor :type Actor%20Object%20Reference) (OtherComp :type Primitive%20Component%20Object%20Reference) (OtherBodyIndex :type Integer))
  (if (Variables|Default|GetNote4Ready)
    (Variables|Default|SetNote4Ready false)))

(event EventBeginPlay
  (bind _returnvalue (Game|GetPlayerController 0))
  (Pawn|UnPossess _returnvalue)
  (Pawn|Possess _returnvalue self)
  (bind _returnvalue_2 (UserInterface|CreateWidget "/Game/Hud/Hud_ATKWidget.Hud_ATKWidget_C"))
  (Variables|Default|SetATK _returnvalue_2)
  (bind _returnvalue_3 (UserInterface|CreateWidget "/Game/Hud/Hud_DEFWidget.Hud_DEFWidget_C"))
  (Variables|Default|SetDEF _returnvalue_3)
  (bind _returnvalue_4 (UserInterface|CreateWidget "/Game/Hud/Hud_EVAWidget.Hud_EVAWidget_C"))
  (Variables|Default|SetEVA _returnvalue_4)
  (UserInterface|Viewport|AddtoViewport (Variables|Default|GetATK) 0))

(event Input|ActionEvents|InputActionNextAction
  (params (Key :type Key%20Structure))
  (:Pressed
    (bind _output_get (Variables|Default|SetWidgetCounter (Math|Integer|%(Integer) (+ (Variables|Default|GetWidgetCounter) 1) 3)))
    (switch int _output_get
      (:0
        (Widget|RemovefromParent (Variables|Default|GetEVA))
        (UserInterface|Viewport|AddtoViewport (Variables|Default|GetATK) 0))
      (:1
        (Widget|RemovefromParent (Variables|Default|GetATK))
        (UserInterface|Viewport|AddtoViewport (Variables|Default|GetDEF) 0))
      (:2
        (Widget|RemovefromParent (Variables|Default|GetDEF))
        (UserInterface|Viewport|AddtoViewport (Variables|Default|GetEVA) 0)))))

(event Input|ActionEvents|InputActionNote2
  (params (Key :type Key%20Structure))
  (:Pressed
    (if (Variables|Default|GetNote2Ready)
      (Development|PrintString "Note2")
      (Variables|Default|SetNote2Ready false))))

(event Input|ActionEvents|InputActionPrevAction
  (params (Key :type Key%20Structure))
  (:Pressed
    (bind _output_get (Variables|Default|SetWidgetCounter (- (Variables|Default|GetWidgetCounter) 1)))
    (if (<= 0 _output_get)
      _
      (else
        (Variables|Default|SetWidgetCounter 2)))
    (switch int (Variables|Default|GetWidgetCounter)
      (:0
        (Widget|RemovefromParent (Variables|Default|GetDEF))
        (UserInterface|Viewport|AddtoViewport (Variables|Default|GetATK) 0))
      (:1
        (Widget|RemovefromParent (Variables|Default|GetEVA))
        (UserInterface|Viewport|AddtoViewport (Variables|Default|GetDEF) 0))
      (:2
        (Widget|RemovefromParent (Variables|Default|GetATK))
        (UserInterface|Viewport|AddtoViewport (Variables|Default|GetEVA) 0)))))

(event Input|ActionEvents|InputActionNote3
  (params (Key :type Key%20Structure))
  (:Pressed
    (if (Variables|Default|GetNote3Ready)
      (Development|PrintString "Note3")
      (Variables|Default|SetNote3Ready false))))

(event Input|ActionEvents|InputActionNote4
  (params (Key :type Key%20Structure))
  (:Pressed
    (if (Variables|Default|GetNote4Ready)
      (Development|PrintString "Note4")
      (Variables|Default|SetNote4Ready false))))

(event Input|ActionEvents|InputActionNote1
  (params (Key :type Key%20Structure))
  (:Pressed
    (if (Variables|Default|GetNote1Ready)
      (Development|PrintString "Note1")
      (Variables|Default|SetNote1Ready false))))

(event Input|KeyboardEvents|S
  (params (Key :type Key%20Structure))
  ;[1 1 1] Spawn 4 notes when 's' is pressed
  (:Pressed
    (bind _returnvalue (Game|SpawnActorfromClass "/Game/DigitalDemon/Blueprints/Notes/Note.Note_C" (Math|Conversions|ToTransform(Vector) (+ (Transformation|GetSocketLocation (Variables|Default|GetNote1Detector) "None") "0, 0,770.000000")) "Undefined" 0 0))
    (Variables|/Game/DigitalDemon/Blueprints/Notes/Note.Note_C|SetendPoint _returnvalue "0, 0,-861.000000")
    (Utilities|FlowControl|Delay 1.0)
    (bind _returnvalue_2 (Game|SpawnActorfromClass "/Game/DigitalDemon/Blueprints/Notes/Note.Note_C" (Math|Conversions|ToTransform(Vector) (+ (Transformation|GetSocketLocation (Variables|Default|GetNote2Detector) "None") "0, 0,770.000000")) "Undefined" 0 0))
    (Variables|/Game/DigitalDemon/Blueprints/Notes/Note.Note_C|SetendPoint _returnvalue_2 "0, 0,-861.000000")
    (Utilities|FlowControl|Delay 1.0)
    (bind _returnvalue_3 (Game|SpawnActorfromClass "/Game/DigitalDemon/Blueprints/Notes/Note.Note_C" (Math|Conversions|ToTransform(Vector) (+ (Transformation|GetSocketLocation (Variables|Default|GetNote3Detector) "None") "0, 0,770.000000")) "Undefined" 0 0))
    (Variables|/Game/DigitalDemon/Blueprints/Notes/Note.Note_C|SetendPoint _returnvalue_3 "0, 0,-861.000000")
    (Utilities|FlowControl|Delay 0.2)
    (bind _returnvalue_4 (Game|SpawnActorfromClass "/Game/DigitalDemon/Blueprints/Notes/Note.Note_C" (Math|Conversions|ToTransform(Vector) (+ (Transformation|GetSocketLocation (Variables|Default|GetNote4Detector) "None") "0, 0,770.000000")) "Undefined" 0 0))
    (Variables|/Game/DigitalDemon/Blueprints/Notes/Note.Note_C|SetendPoint _returnvalue_4 "0, 0,-861.000000")))

(fn ConstructionScript)