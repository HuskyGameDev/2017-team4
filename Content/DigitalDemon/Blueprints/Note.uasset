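; Note Blueprint for a moving note object, driven along a timeline whose play rate is set from the inverse of Speed on BeginPlay.
; MovingForward plays FallTimeline, lerping the Note component's relative location, though both lerp endpoints are zero here.
; When the timeline finishes, it spawns a replacement at the owner's transform, passes on EndPoint, and destroys only its own Note component.
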(event Custom|Moving%20Forward
  ;[1 1 1] Movement Control
  (bind _newtrack_0 (Timeline|FallTimeline PlayFromStart)
    (:Update
      (Transformation|SetRelativeLocation (Variables|Default|GetNote) (Math|Vector|Lerp(Vector) "0, 0, 0" "0, 0, 0" _newtrack_0) false false))
    (:Finished
      (bind _returnvalue (Game|SpawnActorfromClass "Note_C" (Transformation|GetActorTransform (Components|GetOwner (Variables|Default|GetNote))) "Undefined" 0 0))
      (Variables|Note_C|SetendPoint _returnvalue (Variables|Default|GetendPoint))
      (Components|DestroyComponent (Variables|Default|GetNote)))))

(event EventBeginPlay
  (Utilities|FlowControl|Sequence
    (:then_1
      (Components|Timeline|SetPlayRate (Variables|Default|GetFallTimeline) (/ 1.0 (Variables|Default|Getspeed)))
      (Variables|Default|SettestEnd true))))

(event Collision|EventActorBeginOverlap
  (params (OtherActor :type Actor%20Object%20Reference)))

(event EventTick
  (params (DeltaSeconds :type Float%20%28single-precision%29)))

(fn ConstructionScript)