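; BP_Checkpoint is a checkpoint trigger actor with an adjustable box and a billboard, apparently unfinished.
; Its construction script sizes the box from ChangeHitBox and sets the billboard sprite based on the CheckPoint flag.
; Any actor overlap creates and casts a new save game object and assigns an empty SaveInfo, but never writes it to a slot.
; BeginPlay only casts the player pawn, and other overlap checks are unwired.
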(event EventBeginPlay
  (Utilities|Casting|CastToCharacter (Game|Player|GetPlayerPawn 0)))

(event Collision|EventActorBeginOverlap
  (params (OtherActor :type Actor%20Object%20Reference))
  (if true
    (bind _returnvalue (SaveGame|CreateSaveGameObject "/Script/Engine.SaveGame"))
    (bind _assave_info (Utilities|Casting|CastTo _returnvalue))
    (Variables|Default|SetSaveInfo 0 _assave_info)))

(fn ConstructionScript
  (Components|Box|SetBoxExtent (Variables|Default|GetBox) (Variables|Default|GetChangeHitBox) true)
  (if (Variables|Default|GetCheckPoint)
    (Rendering|Components|Sprite|SetSprite (Variables|Default|GetBillboard) 0)
    (else
      (Rendering|Components|Sprite|SetSprite (Variables|Default|GetBillboard) 0))))