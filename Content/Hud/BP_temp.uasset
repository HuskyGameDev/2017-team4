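; BP_temp is an actor Blueprint that sets up the DigitalDemonSave save game.
; On BeginPlay it loads slot DigitalDemonSave if it exists, otherwise creates a save object and writes it to that slot.
; Either path stores the object in SaveGameConnections and casts it to DigitalDemonSave.
; Reads of score, level completion, unlock and name fields are left unconnected and never run.
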(event EventBeginPlay
  ;[1 1 1] Save Game Function
  (bind _returnvalue (SaveGame|DoesSaveGameExist "DigitalDemonSave"))
  (if _returnvalue
    (bind _returnvalue_2 (SaveGame|LoadGamefromSlot "DigitalDemonSave"))
    (Variables|Default|SetSaveGameConnections _returnvalue_2)
    (bind _asdigital_demon_save (Utilities|Casting|CastToDigitalDemonSave (Variables|Default|GetSaveGameConnections)))
    (else
      (bind _returnvalue_3 (SaveGame|CreateSaveGameObject "/Game/Hud/DigitalDemonSave.DigitalDemonSave_C"))
      (Variables|Default|SetSaveGameConnections _returnvalue_3)
      (bind _asdigital_demon_save_2 (Utilities|Casting|CastToDigitalDemonSave (Variables|Default|GetSaveGameConnections)))
      (SaveGame|SaveGametoSlot _asdigital_demon_save_2 "DigitalDemonSave"))))

(event Collision|EventActorBeginOverlap
  (params (OtherActor :type Actor%20Object%20Reference)))

(event EventTick
  (params (DeltaSeconds :type Float%20%28single-precision%29)))

(fn ConstructionScript)